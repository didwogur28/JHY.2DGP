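; Stage 04 pressure button that reacts when something enters or leaves its trigger, demonstrating multicast events.
; Begin overlap calls ButtonPressed, commented as multicast to all clients, which lowers the mesh, lights its emissive and spawns a particle burst.
; End overlap calls ButtonReleased to raise it and clear the glow, using a dynamic material created in the Construction Script.
; Placeholder-named rotation helpers wrap SetRelativeRotation but are unused by the button logic.
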(event `self.Trigger.OnComponentBeginOverlap`
  (params (OverlappedComponent :type "PrimitiveComponent Object Reference") (OtherActor :type "Actor Object Reference") (OtherComp :type "PrimitiveComponent Object Reference") (OtherBodyIndex :type Integer) (bFromSweep :type Boolean) (SweepResult :type "HitResult Structure (by ref)"))
  (`self.Button pressed`) ; Calls a custom event with a sequence for pressing the button
)

(event `self.Trigger.OnComponentEndOverlap`
  (params (OverlappedComponent :type "PrimitiveComponent Object Reference") (OtherActor :type "Actor Object Reference") (OtherComp :type "PrimitiveComponent Object Reference") (OtherBodyIndex :type Integer))
  (`self.Button released`) ; Calls a custom event with a sequence for popping the button back up
)

(event `Button pressed`
  (`SceneComponent.K2_SetRelativeLocation` (`self.Button`) (`KismetMathLibrary.MakeVector` 0.0 0.0 -10.0) false false) ; Move button down
  (`MaterialInstanceDynamic.SetVectorParameterValue` (`self.Button material`) "Emissive" (struct :`R` 5.0 :`G` 3.721064 :`A` 1.0)) ; Change emissive color of the button
  (`GameplayStatics.SpawnEmitterAttached` "/Game/ExampleContent/NetworkFeatures/Effects/P_Particle_Burst.P_Particle_Burst" null "None" (0.0 15.0 0.0)) ; Spawn particle burst
)

(event `Button released`
  (`SceneComponent.K2_SetRelativeLocation` (`self.Button`) (`KismetMathLibrary.MakeVector` 0.0 0.0 0.0) false false) ; Move button up
  (`MaterialInstanceDynamic.SetVectorParameterValue` (`self.Button material`) "Emissive" (struct :`A` 1.0)) ; Change emissive color of the button
)

(fn `NewFunction_0`
  (params (self2 :type "SceneComponent Object Reference") (NewRotation :type "Rotator Structure"))
  (`SceneComponent.K2_SetRelativeRotation` self2 NewRotation false false))

(fn `NewFunction_1`
  (params (self2 :type "SceneComponent Object Reference") (NewRotation :type "Rotator Structure"))
  (`self.NewMacro_0` self2 NewRotation))

(fn `UserConstructionScript`
  (bind _returnvalue (`PrimitiveComponent.CreateDynamicMaterialInstance` (`self.Button`) 0 null)) ; Make and apply a dynamic material instance for the button
  (set `self.Button material` _returnvalue) ; Set the material as a variable for animating
)